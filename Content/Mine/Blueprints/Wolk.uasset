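; Wolk is a player-controlled pawn with axis-driven movement and look, which hands control to the first Ia actor on F.
; Forward and Right feed movement input along E's negated horizontal axes, which Tick consumes as an unswept local offset.
; X disables Tick, halting movement, and Z re-enables it; both also drive a Gate node.
; Turn and look-up axes each have two handlers, one rate-scaled by delta time and one raw.
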(event `Key|S`
  (params (Key :type "Key Structure")))

(event `Key|W`
  (params (Key :type "Key Structure")))

(event `Key|X`
  (params (Key :type "Key Structure"))
  (:`Pressed`
    (`/Engine/EditorBlueprintResources/StandardMacros.Gate` true :!via `Open` :!label _label
      (:`Exit`
        (`KismetSystemLibrary.PrintString` "The Gates Are Open!")))))

(event `Key|A`
  (params (Key :type "Key Structure")))

(event `Key|Z`
  (params (Key :type "Key Structure"))
  (:`Pressed`
    (goto _label :!via `Close`)))

(event `Key|D`
  (params (Key :type "Key Structure")))

(event `Key|X`
  (params (Key :type "Key Structure"))
  (:`Pressed`
    (`self.SetActorTickInterval` 0.0)
    (`self.SetActorTickEnabled` false)))

(event `Key|Z`
  (params (Key :type "Key Structure"))
  (:`Pressed`
    (`self.SetActorTickInterval` 0.0)
    (`self.SetActorTickEnabled` true)))

(event `self.ReceiveTick`
  (params (DeltaSeconds :type "Float (single-precision)"))
  (bind _returnvalue (`self.ConsumeMovementInputVector`))
  (`self.K2_AddActorLocalOffset` _returnvalue))

(event `InputAxis|RateTurn`
  (params (AxisValue :type "Float (single-precision)"))
  (`self.AddControllerYawInput` (* AxisValue (`self.BTR`) (`GameplayStatics.GetWorldDeltaSeconds`))))

(event `InputAxis|Forward`
  (params (AxisValue :type "Float (single-precision)"))
  (`self.AddMovementInput` (* (`SceneComponent.GetForwardVector` (`self.e`)) (-10.0 -10.0 0.0)) AxisValue))

(event `InputAxis|RateUp`
  (params (AxisValue :type "Float (single-precision)"))
  (`self.AddControllerPitchInput` (* AxisValue (`self.BLUP`) (`GameplayStatics.GetWorldDeltaSeconds`))))

(event `InputAxis|RateTurn`
  (params (AxisValue :type "Float (single-precision)"))
  (`self.AddControllerYawInput` AxisValue))

(event `InputAxis|Right`
  (params (AxisValue :type "Float (single-precision)"))
  (`self.AddMovementInput` (* (`SceneComponent.GetRightVector` (`self.e`)) (-10.0 -10.0 0.0)) AxisValue))

(event `InputAxis|RateUp`
  (params (AxisValue :type "Float (single-precision)"))
  (`self.AddControllerPitchInput` AxisValue))

(event `Key|F`
  (params (Key :type "Key Structure"))
  (:`Pressed`
    (bind _outactors (`GameplayStatics.GetAllActorsOfClass` "/Game/Mine/Blueprints/Ia.Ia_C"))
    (`Controller.Possess` (`GameplayStatics.GetPlayerController` 0) (`|GetArrayItem` _outactors))))

(fn `UserConstructionScript`)