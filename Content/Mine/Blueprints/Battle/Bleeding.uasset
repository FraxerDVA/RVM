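; Bleeding Blueprint that applies damage over time to a target object in battle.
; Bleed passes the target to the WaitForBleed event, which calls the target's Damage at one-second intervals with a small fixed amount.
; A custom LoopWithDelay macro paces the hits as a latent counting loop with an inclusive upper bound.
; An unconnected fire storm spawn remains in Bleed and never runs.
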(event `WaitForBleed`
  (params (Obj :type "/Game/Mine/Blueprints/CharactersStats Object Reference"))
  (bind _index (`self.LoopWithDelay` 0 12 1.0)
    (:`LoopBody`
      (`/Game/Mine/Blueprints/CharactersStats.Damage` Obj 1.5 Obj))))

(fn `Bleed`
  (params (Object :type "/Game/Mine/Blueprints/CharactersStats Object Reference"))
  (`self.WaitForBleed` Object))