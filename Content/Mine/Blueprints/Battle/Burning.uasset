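; Burning is a battle Blueprint that applies burn damage over time to a given object.
; Burn hands the object to the Wait event, which deals a small hit each second for twenty seconds, then clears the object's IsBurning flag.
; A custom LoopWithDelay macro spaces the hits with a latent Delay between iterations.
; Fire emitter and firestorm spawn nodes sit unconnected in Burn, so no visual effect spawns.
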(event `Wait`
  (params (Obj :type "/Game/Mine/Blueprints/CharactersStats Object Reference"))
  (bind _index (`self.LoopWithDelay` 0 19 1.0)
    (:`LoopBody`
      (`/Game/Mine/Blueprints/CharactersStats.Damage` Obj 1.0 Obj)
      (`KismetSystemLibrary.PrintString` (`KismetStringLibrary.Conv_IntToString` _index)))
    (:`Completed`
      (set `/Game/Mine/Blueprints/CharactersStats.IsBurning` false Obj))))

(event `self.ReceiveBeginPlay`)

(fn `Burn`
  (params (Object :type "/Game/Mine/Blueprints/CharactersStats Object Reference"))
  (`self.Wait` Object))