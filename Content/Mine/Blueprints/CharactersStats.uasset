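; CharactersStats holds a character's health, stamina and magicka, along with a battle flag and a profile picture number for the HUD target display.
; Functions fill stats to their maximums, deduct stamina or magicka costs, and regenerate both by fixed steps per call.
; Damage lowers health and flags battle; on death it zeroes stamina, magicka and their maximums, then calls EnemyCallMessage on the passed object.
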(event `self.ReceiveBeginPlay`)

(event `self.ReceiveTick`
  (params (DeltaSeconds :type "Float (single-precision)")))

(fn `Damage`
  (params (TakenDamage :type "Float (double-precision)") (Obj :type "Actor Object Reference"))
  (if (> (`self.Health`) 0.0)
    (bind _output_get (set `self.Health` (- (`self.Health`) TakenDamage)))
    (set `self.BattleOn` true)
    (if (<= _output_get 0.0)
      (set `self.Magicka` 0.0)
      (set `self.Stamina` 0.0)
      (set `self.MaxMagicka` 0.0)
      (set `self.MaxStamina` 0.0)
      (message `/Game/Mine/Blueprints/BPC.EnemyCall` Obj))))

(fn `Is Dead`
  (returns (NewParam :type Boolean))
  (return (<= (`self.Health`) 0.0)))

(fn `RecoveryStaminaAndMagicka`
  (if (< (`self.Stamina`) (`self.MaxStamina`))
    (set `self.Stamina` (+ (`self.Stamina`) 1.0)))
  (if (< (`self.Magicka`) (`self.MaxMagicka`))
    (set `self.Magicka` (+ (`self.Magicka`) 1.0))))

(fn `SetHpStMg`
  (set `self.Health` (`self.MaxHealth`))
  (set `self.Stamina` (`self.MaxStamina`))
  (set `self.Magicka` (`self.MaxMagicka`)))

(fn `SetProfPic`
  (params (HUD :type "/Game/Mine/UI/HUD Object Reference"))
  (`/Game/Mine/UI/HUD.SetTargetPic` HUD (`self.NumberOfProfilePictue`)))

(fn `StaminaOrMagickPrice`
  (params (Stamina :type Boolean) (Cost :type "Float (double-precision)"))
  (if Stamina
    (set `self.Stamina` (- (`self.Stamina`) Cost))
    (else
      (set `self.Magicka` (- (`self.Magicka`) Cost)))))

(fn `UserConstructionScript`)