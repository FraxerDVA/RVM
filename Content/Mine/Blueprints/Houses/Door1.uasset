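; Door actor for the houses that toggles between open and closed by rotating itself.
; DoorOpen2, with no caller in this graph, starts a fast looping timer on StartOpen, which adds a small local rotation step each tick, signed by the Open flag.
; A Delay of just under a second ends the swing by flipping Open and clearing the timer, so motion is timed rather than angle-checked.
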(event `/Game/Mine/Blueprints/BPC.DoorOpen2`
  (`self.StartOpen`)
  (bind _returnvalue (`KismetSystemLibrary.K2_SetTimerDelegate` (delegate `StartOpen`) 0.01 true)))

(event `StartOpen`
  (if (`self.Open`)
    (`self.K2_AddActorLocalRotation` (`|EaseFunction` "Step" 1.0 (`self.K2_GetActorRotation`) (struct :`Yaw` 1.0) true 10))
    (`KismetSystemLibrary.Delay` 0.95)
    (set `self.Open` false)
    (else
      (`self.K2_AddActorLocalRotation` (`|EaseFunction` "Step" 1.0 (`self.K2_GetActorRotation`) (struct :`Yaw` -1.0) true 10))
      (`KismetSystemLibrary.Delay` 0.95)
      (set `self.Open` true)))
  (`KismetSystemLibrary.K2_ClearAndInvalidateTimerHandle` (stale `/Game/Mine/Blueprints/BPC.DoorOpen2` _returnvalue)))

(event `self.ReceiveTick`
  (params (DeltaSeconds :type "Float (single-precision)")))

(fn `UserConstructionScript`)