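; QuestLibrary provides MakeRandomQuest, which generates a randomized quest with Russian display text.
; Only one template exists so far, a wolf-hunting order, as both random selectors are pinned to a single value and the other target slot is a placeholder.
; It rolls a kill count, scales gold and experience from it, and returns title, description, reward and progress text alongside the raw quest data.
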(fn `MakeRandomQuest`
  (returns (SetTittle :type Text) (SetDescription :type Text) (SetReward :type Text) (TargetCountExt :type Integer) (QuestTypeExt :type Integer) (RewardGoldExt :type Integer) (RewardExpExt :type Integer) (TargetTypeExt :type String) (ActiveDesc :type String))
  (locals (Tittle :type Text) (Description :type Text) (Reward :type Text) (TargetCount :type Integer) (QuestType :type Integer) (RewardGold :type Integer) (RewardExp :type Integer) (TargetType :type String) (TargetTypeInt :type Integer))
  (switch `int` (`KismetMathLibrary.RandomIntegerInRange` 0)
    (:`0`
      (set `local.QuestType` 1)
      (set `local.TargetTypeInt` (`KismetMathLibrary.RandomIntegerInRange` 1 1))
      (bind _output_get (set `local.TargetType` (`|GetArrayItem` (`|MakeArray` "Potom Pridymau" "Wolf") (`local.TargetTypeInt`))))
      (bind _output_get_2 (set `local.TargetCount` (`KismetMathLibrary.RandomIntegerInRange` 3 8)))
      (set `local.RewardGold` (* _output_get_2 20))
      (set `local.RewardExp` (* _output_get_2 15))
      (set `local.Tittle` (`KismetTextLibrary.Conv_StringToText` (`KismetStringLibrary.Concat_StrStr` "Заказ: " (`|GetArrayItem` (`|MakeArray` "Potom Pridymau" "Волки") (`local.TargetTypeInt`)))))
      (set `local.Description` (`KismetTextLibrary.Conv_StringToText` (`KismetStringLibrary.BuildString_Int` "Требуется убить " "" _output_get_2 (`KismetStringLibrary.Concat_StrStr` (`|GetArrayItem` (`|MakeArray` " Potom Pridymau" " волков") (`local.TargetTypeInt`)) " в окрестных лесах."))))
      (set `local.Reward` (`KismetTextLibrary.Conv_StringToText` (`KismetStringLibrary.BuildString_Int` (`KismetStringLibrary.BuildString_Int` "Награда: " "" (`local.RewardGold`) " золота") " \n" (`local.RewardExp`) " Очков Опыта")))
      (return (`local.Tittle`) (`local.Description`) (`local.Reward`) (`local.TargetCount`) (`local.QuestType`) (`local.RewardGold`) (`local.RewardExp`) _output_get (`KismetStringLibrary.BuildString_Int` (`|GetArrayItem` (`|MakeArray` " Potom Pridymau" " Волки: 0/") (`local.TargetTypeInt`)) "" (`local.TargetCount`))))))