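; Quest bill board actor that hands out random quests and pays gold and experience on completion.
; Interacting shows a newly generated quest when free, the current one when taken, or a completion notice.
; Accepting adds a quest component to the player and starts it with the generated parameters; accepting when complete rewards and removes it.
; Focus briefly outlines the board meshes via custom depth, cleared by a retriggerable delay.
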(event `/Game/Mine/Blueprints/BPC.InteractiveObject`
  (params (HUD :type "/Game/Mine/UI/HUD Object Reference") (Player :type "/Game/Mine/Blueprints/MainPlayer Object Reference"))
  (if (`self.QuestComplete`)
    (`/Game/Mine/UI/HUD.ShowAgreeQuest` HUD)
    (`/Game/Mine/UI/HUD.QuestOn` HUD self (stale `/Game/Mine/Blueprints/BPC.InteractiveObject` _settittle) "Выполнено" (stale _setreward))
    (elif (`self.NeZanyat`)
      (bind (_settittle _setdescription _setreward _targetcountext _questtypeext _rewardgoldext _rewardexpext _targettypeext _activedesc) (`/Game/Mine/Blueprints/Quests/QuestLibrary.MakeRandomQuest`))
      (`/Game/Mine/UI/HUD.QuestOn` HUD self _settittle _setdescription _setreward)
      (else
        (`/Game/Mine/UI/HUD.HideAgreeQuest` HUD)
        (`/Game/Mine/UI/HUD.QuestOn` HUD self _settittle _setdescription _setreward)))))

(event `/Game/Mine/Blueprints/BPC.Answer`
  (params (Agree :type Boolean))
  (if Agree
    (if (`self.QuestComplete`)
      (set `self.NeZanyat` true)
      (set `self.QuestComplete` false)
      (set `/Game/Mine/Blueprints/MainPlayer.GoldCount` (+ (`/Game/Mine/Blueprints/MainPlayer.GoldCount` (stale `/Game/Mine/Blueprints/BPC.InteractiveObject` Player)) (stale `/Game/Mine/Blueprints/BPC.InteractiveObject` _rewardgoldext)) (stale `/Game/Mine/Blueprints/BPC.InteractiveObject` Player))
      (set `/Game/Mine/Blueprints/MainPlayer.ExperienceCount` (+ (`/Game/Mine/Blueprints/MainPlayer.ExperienceCount` (stale `/Game/Mine/Blueprints/BPC.InteractiveObject` Player)) (stale `/Game/Mine/Blueprints/BPC.InteractiveObject` _rewardexpext)) (stale `/Game/Mine/Blueprints/BPC.InteractiveObject` Player))
      (`ActorComponent.K2_DestroyComponent` (stale _returnvalue))
      (`/Game/Mine/UI/HUD.ShowActiveQuest` (stale `/Game/Mine/Blueprints/BPC.InteractiveObject` HUD) "" "")
      (bind _questsarray (`/Game/Mine/Blueprints/MainPlayer.QuestsArray` (stale `/Game/Mine/Blueprints/BPC.InteractiveObject` Player)))
      (`KismetArrayLibrary.Array_RemoveItem` _questsarray (stale _returnvalue))
      (else
        (set `self.NeZanyat` false)
        (set `self.QuestComplete` false)
        (bind _returnvalue (`AddComponent|NODE_AddQuestComponent-0` :`self` (stale `/Game/Mine/Blueprints/BPC.InteractiveObject` Player)))
        (`/Game/Mine/UI/HUD.ShowActiveQuest` (stale `/Game/Mine/Blueprints/BPC.InteractiveObject` HUD) (stale `/Game/Mine/Blueprints/BPC.InteractiveObject` _settittle) (`KismetTextLibrary.Conv_StringToText` (stale `/Game/Mine/Blueprints/BPC.InteractiveObject` _activedesc)))
        (`KismetArrayLibrary.Array_Add` _questsarray _returnvalue)
        (`/Game/Mine/Blueprints/Quests/QuestComponent.StartQuest` _returnvalue (stale `/Game/Mine/Blueprints/BPC.InteractiveObject` _targetcountext) (stale `/Game/Mine/Blueprints/BPC.InteractiveObject` _questtypeext) (stale `/Game/Mine/Blueprints/BPC.InteractiveObject` _targettypeext) (`KismetTextLibrary.Conv_TextToString` (stale `/Game/Mine/Blueprints/BPC.InteractiveObject` _settittle)) (stale `/Game/Mine/Blueprints/BPC.InteractiveObject` HUD) self)))))

(event `/Game/Mine/Blueprints/BPC.OnFocus`
  (`PrimitiveComponent.SetRenderCustomDepth` (`self.BillBoard`) true)
  (`PrimitiveComponent.SetRenderCustomDepth` (`self.List1`) true)
  (`PrimitiveComponent.SetRenderCustomDepth` (`self.List2`) true)
  (`PrimitiveComponent.SetRenderCustomDepth` (`self.List3`) true)
  (`PrimitiveComponent.SetRenderCustomDepth` (`self.List4`) true)
  (`PrimitiveComponent.SetRenderCustomDepth` (`self.List5`) true)
  (`PrimitiveComponent.SetRenderCustomDepth` (`self.List`) true)
  (bind _output_get (set `self.Timer` 0.1))
  (`KismetSystemLibrary.RetriggerableDelay` _output_get)
  (`PrimitiveComponent.SetRenderCustomDepth` (`self.List`) false)
  (`PrimitiveComponent.SetRenderCustomDepth` (`self.List5`) false)
  (`PrimitiveComponent.SetRenderCustomDepth` (`self.List4`) false)
  (`PrimitiveComponent.SetRenderCustomDepth` (`self.List3`) false)
  (`PrimitiveComponent.SetRenderCustomDepth` (`self.List2`) false)
  (`PrimitiveComponent.SetRenderCustomDepth` (`self.List1`) false)
  (`PrimitiveComponent.SetRenderCustomDepth` (`self.BillBoard`) false))

(fn `UserConstructionScript`)