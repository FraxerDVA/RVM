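; MapPlayer is a player Blueprint that provides click-to-move navigation.
; On a left mouse press it traces under the cursor against WorldStatic objects, prints the hit point raised slightly in Z, and sends the player controller there with SimpleMoveToLocation.
; Other events are empty, and several alternative movement and cursor-projection experiments are left disconnected.
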(event `Key|LeftMouseButton`
  (params (Key :type "Key Structure"))
  (bind _returnvalue (`KismetMathLibrary.MakeVector` (.x (`.Location` (`GameplayStatics.BreakHitResult` (`PlayerController.GetHitResultUnderCursorForObjects` (`GameplayStatics.GetPlayerController` 0) (`|MakeArray` "ObjectTypeQuery1" :!type "EObjectTypeQuery Enum") true)))) (.y (`.Location` (`GameplayStatics.BreakHitResult` (`PlayerController.GetHitResultUnderCursorForObjects` (`GameplayStatics.GetPlayerController` 0) (`|MakeArray` "ObjectTypeQuery1" :!type "EObjectTypeQuery Enum") true)))) (+ (.z (`.Location` (`GameplayStatics.BreakHitResult` (`PlayerController.GetHitResultUnderCursorForObjects` (`GameplayStatics.GetPlayerController` 0) (`|MakeArray` "ObjectTypeQuery1" :!type "EObjectTypeQuery Enum") true)))) 1.0)))
  (:`Pressed`
    (`KismetSystemLibrary.PrintString` (`KismetStringLibrary.Conv_VectorToString` _returnvalue))
    (`AIBlueprintHelperLibrary.SimpleMoveToLocation` (`GameplayStatics.GetPlayerController` 0) _returnvalue)))

(event `self.ReceiveBeginPlay`)

(event `InputAxisKey|MouseWheelAxis`
  (params (AxisValue :type "Float (single-precision)")))

(event `self.ReceiveTick`
  (params (DeltaSeconds :type "Float (single-precision)")))

(fn `UserConstructionScript`)